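; BP_PatrolRoute is a spline-based patrol path for AI that supplies one world-space waypoint at a time.
; IncrementPatrolRoute steps CurIndex along the PatrolRoute spline points, flipping Direction at the last and first points so the route runs back and forth instead of looping.
; GetSplinePointLocation returns the world location of the spline point at CurIndex.
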(event `IncrementPatrolRoute`
  (bind _output_get (set `self.CurIndex` (+ (`self.CurIndex`) (`self.Direction`))))
  (if (== _output_get (- (`SplineComponent.GetNumberOfSplinePoints` (`self.PatrolRoute`)) 1))
    (set `self.Direction` -1)
    (elif (== (`self.CurIndex`) 0)
      (set `self.Direction` 1))))

(fn `GetSplinePointLocation`
  (returns (Location :type "Vector Structure"))
  (return (`SplineComponent.GetLocationAtSplinePoint` (`self.PatrolRoute`) (`self.CurIndex`) "World")))

(fn `UserConstructionScript`)