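; BPC_DamageSystem is a component that resolves incoming damage and healing against a health component passed into each call.
; TakeDamage uses the CanBeDamaged macro to branch on death, invincibility and blocking, returning true only when damage lands.
; It fires dispatchers for block, death and damage response, the last only if interruptible or forced.
; Heal adds a fraction of max health while alive.
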(fn `Heal`
  (params (Amount :type "Float (double-precision)") (HealthComp :type "Object Object Reference"))
  (returns (NewHealth :type "Float (double-precision)"))
  (bind _maxhealth (`/Game/_DevContent_/DamageSystem/BPC_DamageSystem.MaxHealth` HealthComp))
  (if (not (`/Game/_DevContent_/DamageSystem/BPC_DamageSystem.IsDead` HealthComp))
    (bind _output_get (set `/Game/_DevContent_/DamageSystem/BPC_DamageSystem.CurHealth` (`KismetMathLibrary.FClamp` (+ (`/Game/_DevContent_/DamageSystem/BPC_DamageSystem.CurHealth` HealthComp) (* Amount _maxhealth)) 0.0 _maxhealth) HealthComp))
    (return _output_get)))

(fn `TakeDamage`
  (params (DamageInfo :type "/Game/_DevContent_/DamageSystem/S_DamageInfo Structure") (HealthComp :type "/Game/_DevContent_/Components/BP_HealthComp Object Reference"))
  (returns (WasDamaged :type Boolean))
  (bind (_amount _damagetype _damageresponse _shoulddamageinvincible _canbeblocked _canbeparried _shouldforceinterrupt) (break `/Game/_DevContent_/DamageSystem/S_DamageInfo` DamageInfo))
  (`self.CanBeDamaged` _shoulddamageinvincible _canbeblocked HealthComp
    (:`BlockDamage`
      (`self.OnBlocked` _canbeparried))
    (:`DoDamage`
      (bind _output_get (set `/Game/_DevContent_/DamageSystem/BPC_DamageSystem.CurHealth` (`KismetMathLibrary.FClamp` (- (`/Game/_DevContent_/DamageSystem/BPC_DamageSystem.CurHealth` HealthComp) _amount) 0.0 (`/Game/_DevContent_/DamageSystem/BPC_DamageSystem.MaxHealth` HealthComp)) HealthComp))
      (if (<= _output_get 0.0)
        (set `/Game/_DevContent_/DamageSystem/BPC_DamageSystem.IsDead` true HealthComp)
        (`self.OnDeath`)
        (elif (or (`self.IsInterruptible`) _shouldforceinterrupt)
          (`self.OnDamageResponse` _damageresponse)))
      (return true))
    (:`NoDamage`
      _))
  (return false))