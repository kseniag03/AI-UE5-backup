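; BP_ManaComp is a component that tracks a mana pool for its owner, used for casting costs.
; BeginPlay caches the owner and fills current mana to a fixed maximum.
; CanCast checks a cost against current mana, and WasteMana subtracts an amount clamped between zero and max, returning the new value.
; A separate event, dd, subtracts mana without clamping, and nothing in the graphs regenerates it.
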(event `self.ReceiveBeginPlay`
  (set `self.Owner` (`self.GetOwner`))
  (bind _output_get (set `self.MaxMana` 100.0))
  (set `self.CurMana` _output_get))

(event `dd`
  (params (Waste :type Integer))
  (set `self.CurMana` (- (`self.CurMana`) Waste)))

(fn `CanCast`
  (params (Cost :type Integer))
  (returns (CanCast :type Boolean))
  (return (<= Cost (`self.CurMana`))))

(fn `WasteMana`
  (params (AmountToWaste :type "Float (double-precision)"))
  (returns (CurMana :type "Float (double-precision)"))
  (bind _output_get (set `self.CurMana` (`KismetMathLibrary.FClamp` (- (`self.CurMana`) AmountToWaste) 0.0 (`self.MaxMana`))))
  (return _output_get))