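; BP_StaminaComp is a stamina component that stores current and maximum stamina for its owner, starting full on BeginPlay.
; WasteStamina and FillStamina adjust the clamped value and return it, with no Tick logic, so callers drive every change.
; Depletion fires the AllStaminaSpent dispatcher and clears CanRun, which FillStamina never restores.
; FillStamina sets CanFill according to whether stamina is below maximum, and WasteStamina debug-prints non-empty values.
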(event `self.ReceiveBeginPlay`
  (set `self.Owner` (`self.GetOwner`))
  (bind _output_get (set `self.MaxStamina` 100.0))
  (set `self.CurStamina` _output_get)
  (set `self.CanRun` true)
  (set `self.CanFill` true))

(fn `FillStamina`
  (params (AmountToFill :type "Float (double-precision)"))
  (returns (CurStamina :type "Float (double-precision)"))
  (bind _output_get (set `self.CurStamina` (`KismetMathLibrary.FClamp` (+ (`self.CurStamina`) AmountToFill) 0.0 (`self.MaxStamina`))))
  (if (>= _output_get (`self.MaxStamina`))
    (set `self.CanFill` false)
    (else
      (set `self.CanFill` true)))
  (return (`self.CurStamina`)))

(fn `WasteStamina`
  (params (AmountToWaste :type "Float (double-precision)"))
  (returns (CurStamina :type "Float (double-precision)"))
  (bind _output_get (set `self.CurStamina` (`KismetMathLibrary.FClamp` (- (`self.CurStamina`) AmountToWaste) 0.0 (`self.MaxStamina`))))
  (if (<= _output_get 0.0)
    (`self.OnAllStaminaSpent`)
    (set `self.CanRun` false)
    (else
      (`KismetSystemLibrary.PrintString` (`KismetStringLibrary.Conv_DoubleToString` _output_get))))
  (return (`self.CurStamina`)))